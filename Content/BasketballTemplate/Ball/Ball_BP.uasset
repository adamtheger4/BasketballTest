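; Basketball actor that handles ownership, pickup, dribbling and shots, moving by scripted lerps.
; On authority, Tick advances the current action unless an interrupting player is in range, otherwise follows the owner's lead hand or checks for pickup.
; Dribbles lerp to a velocity-predicted point, then home back to the hand.
; Shots release ownership and follow an arced path joined to the hoop's path, firing an event at the success point.
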(event Custom|BlockChangeOwnerFor
  (params (Time :type Float%20%28single-precision%29))
  ;[1 1 1] block possibility to change owner for
  (Variables|Default|SetBlockChangeOwner true)
  (Utilities|Time|ClearandInvalidateTimerbyHandle (Variables|Default|GetBlockChangeOwnerTimeHandle))
  (bind _returnvalue (Utilities|Time|SetTimerbyEvent (delegate Custom|RemoveBouncingBlock) Time))
  (Variables|Default|SetBlockChangeOwnerTimeHandle _returnvalue))

(event Custom|ProccedShot
  ;[1 0.471 0] proceed shot (called every frame during shot)
  (if (not (>= (Variables|CurvedTemp|GetCurrentCurvedPathIndex) (- (Utilities|Array|Length (Variables|CurvedTemp|GetСurvedPathData)) 1)))
    (CallFunction|MovementStraightRoutine (Utilities|Array|Get(acopy) (Variables|CurvedTemp|GetСurvedPathData) (Variables|CurvedTemp|GetCurrentCurvedPathIndex)) (Utilities|Array|Get(acopy) (Variables|CurvedTemp|GetСurvedPathData) (+ (Variables|CurvedTemp|GetCurrentCurvedPathIndex) 1)))
    (if (>= (Variables|Temp|GetTempAlpha) 1.0)
      ;;[1 1 1] discard temps
      (Variables|Temp|SetTempAlpha 0.0)
      (Variables|Temp|SetStartPosition (Transformation|GetActorLocation))
      (bind _result (Math|Integer|IncrementInt (Variables|CurvedTemp|GetCurrentCurvedPathIndex))
        (:%20%20
          (Utilities|RecalculateSpeedforPathPair _result)
          ;;[1 1 1] check success shot
          (if (!= (Variables|CurvedTemp|GetIndexOfSuccessShot) -1)
            (if (>= (Variables|CurvedTemp|GetCurrentCurvedPathIndex) (Variables|CurvedTemp|GetIndexOfSuccessShot))
              (Variables|CurvedTemp|SetIndexOfSuccessShot -1)
              (Default|CallOnSuccessPointReached (Variables|Default|GetShotFromActor) (Variables|Default|GetShotFromDistance)))))))
    (else
      (Variables|Default|SetCurrentActionType "NewEnumerator6")
      (Default|CallOnShotDone)
      (Default|CallOnActionDone)
      (EventDispatchers|UnbindallEventsfromOnActionDone))))

(event Custom|CheckToPickFreeBall
  ;[1 1 1] check to pick free ball
  (bind _actor (CallFunction|GetNearestPlayer))
  (bind _canpick (CallFunction|CanbePickedUp _actor))
  (if _canpick
    (CallFunction|SetBallOwner _actor)))

(event Custom|ProccedSelfSpaceBounce
  (bind _ballowner (Variables|Default|GetBallOwner))
  (bind _ballowner_2 (Variables|Default|GetBallOwner))
  ;[1 0.471 0] procced self space bounce (Called every frame during bounce)
  (if (Variables|Temp|GetBounceDown)
    (CallFunction|MovementStraightRoutine (Variables|Temp|GetStartPosition) (Variables|Temp|GetPredictedEndPosition))
    (if (>= (Variables|Temp|GetTempAlpha) 1.0)
      ;;[1 1 1] discard temps
      (Variables|Temp|SetTempAlpha 0.0)
      (Variables|Temp|SetStartPosition (Transformation|GetActorLocation))
      ;;[1 1 1] change direction of bounce
      (Variables|Temp|SetBounceDown false)
      ;;[1 1 1] calculate predicted end position
      ;;;[1 1 1] add owner check
      (Utilities|IsValid _ballowner
        (:Is%20Valid
          (bind _value (Class|SocketUtilsInterfaceBP|GetHandLocation(Message) _ballowner (Variables|Temp|GetBounceFinishHand)))
          (Variables|Temp|SetPredictedEndPosition (+ _value (* (Variables|Temp|GetMovementDirection) (Variables|Temp|GetMovementSpeedMultiplier)))))))
    (else
      (bind _value_2 (Class|SocketUtilsInterfaceBP|GetLeadHand(Message) _ballowner_2))
      (CallFunction|MovementtoHandRoutine _ballowner_2 _value_2 (Variables|Temp|GetStartPosition) (Variables|Temp|GetPredictedEndPosition))
      (if (>= (Variables|Temp|GetTempAlpha) 1.0)
        (Variables|Default|SetCurrentActionType "NewEnumerator6")
        (Default|CallOnActionDone)
        (EventDispatchers|UnbindallEventsfromOnActionDone)))))

(event Custom|StartSelfSpaceBounce
  (params (Duration :type Float%20%28single-precision%29) (MovementSpeed :type Float%20%28single-precision%29) (MovementDirection :type Vector) (MaxSpeed :type Float%20%28single-precision%29))
  (bind _ballowner (Variables|Default|GetBallOwner))
  ;[0.9516 0.7001 1] starters
  ;;[1 0.471 0] start self space bounce
  (if (not (CallFunction|IsBusy))
    (bind _value (Class|SocketUtilsInterfaceBP|GetLeadHand(Message) _ballowner))
    (bind _distance (Class|SocketUtilsInterfaceBP|GetDistanceBetweenRootandHand(Message) _ballowner _value))
    (CallFunction|StartBounce (CallFunction|GetPositionBallBouncefrom) Duration _distance MovementSpeed MovementDirection _value _value MaxSpeed (Variables|Default|GetBallOwner))
    (Variables|Temp|SetBounceDown true)
    (Variables|Default|SetCurrentActionType "NewEnumerator4")))

(event Custom|MovementProccessing
  ;[1 1 1] movement processing
  (Variables|Temp|SetTempAlpha (Math|Float|Clamp(Float) (+ (Variables|Temp|GetTempAlpha) (* (Variables|Temp|GetSpeed) (Utilities|Time|GetWorldDeltaSeconds)))))
  (switch Utilities|FlowControl|Switch|SwitchonEBallActionType (Variables|Default|GetCurrentActionType)
    (:NewEnumerator4
      (CallFunction|ProccedSelfSpaceBounce :!label _label))
    (:NewEnumerator5
      (goto _label))
    (:NewEnumerator7
      (CallFunction|ProccedShot))))

(event Custom|RemoveBouncingBlock
  ;[1 1 1] block possibility to change owner for
  (Variables|Default|SetBlockChangeOwner false))

(event Custom|StartShot
  (params (FromActor :type Actor%20Object%20Reference) (TargetHoop :type Actor%20Object%20Reference) (Duration :type Float%20%28single-precision%29) (PerDistance :type Float%20%28single-precision%29))
  ;[0.9516 0.7001 1] starters
  ;;[1 0.471 0] start shot
  (Variables|Temp|SetDuration Duration)
  (Variables|Temp|SetDistance PerDistance)
  (Variables|Default|SetShotFromActor FromActor)
  (Variables|Default|SetShotFromDistance (Transformation|GetDistanceTo FromActor TargetHoop))
  (bind _value (Class|SocketUtilsInterfaceBP|GetLeadHandLocation(Message) FromActor))
  (Variables|Temp|SetStartPosition _value)
  (bind (_path _successindex) (Class|HoopInterfaceBP|GetPathDatafor(Message) TargetHoop FromActor))
  (bind _path_2 (CallFunction|CurvePath (Variables|Temp|GetStartPosition) (Utilities|Array|Get(acopy) _path) 5 "0, 0,50.000000"))
  (bind _output_get (Variables|CurvedTemp|SetСurvedPathData _path_2))
  (Utilities|RecalculateSpeed (Math|Vector|Distance(Vector) (Utilities|Array|Get(acopy) _output_get) (Utilities|Array|Get(acopy) _output_get 1)))
  (Utilities|FlowControl|Sequence
    (:then_0
      ;;;[1 1 1] for checking what we done success shot point
      (if (!= _successindex -1)
        (Variables|CurvedTemp|SetIndexOfSuccessShot (+ (- (Utilities|Array|Length _path_2) 1) _successindex))
        (else
          (Variables|CurvedTemp|SetIndexOfSuccessShot -1))))
    (:then_1
      ;;;[1 1 1] thats already in path by CurvePath
      (Utilities|Array|RemoveIndex _path)
      (Utilities|AppendPathtoCurrentCurvedPath _path)
      ;;;[1 1 1] discard temp
      (Variables|Temp|SetTempAlpha 0.0)
      (Variables|CurvedTemp|SetCurrentCurvedPathIndex 0)
      (CallFunction|SetBallOwner)
      (Variables|Default|SetCurrentActionType "NewEnumerator7")
      (Default|CallOnShotStart))))

(event Custom|ClientOnOwnerChanged
  (params (NewOwner :type Actor%20Object%20Reference))
  (Default|CallOnOwnerChanged NewOwner))

(event Custom|MovementToHand_Routine
  (params (TargetActor :type Actor%20Object%20Reference) (TargetActorHand :type ELeadHand%20Enum :default "NewEnumerator0") (StartPosition :type Vector) (PredictedEndPosition :type Vector))
  ;[1 1 1] movement to hand: for ends of movement where we want to move toward to hand
  (bind _value (Class|SocketUtilsInterfaceBP|GetHandLocation(Message) TargetActor TargetActorHand))
  (Transformation|SetActorLocation (Math|Vector|Lerp(Vector) StartPosition (Math|Vector|Lerp(Vector) PredictedEndPosition _value (Variables|Temp|GetTempAlpha)) (Variables|Temp|GetTempAlpha)) false true))

(event Custom|MovementStraight_Routine
  (params (StartPosition :type Vector) (EndPosition :type Vector))
  ;[1 1 1] Movement straight : for point to point movements
  (Transformation|SetActorLocation (Math|Vector|Lerp(Vector) StartPosition EndPosition (Variables|Temp|GetTempAlpha)) false true))

(event Custom|BallFollowing
  (bind _ballowner (Variables|Default|GetBallOwner))
  ;[1 1 1] ball following
  (Utilities|IsValid _ballowner
    (:Is%20Valid
      (bind _value (Class|SocketUtilsInterfaceBP|GetLeadHandLocation(Message) _ballowner))
      (Transformation|SetActorLocation _value false true))))

(event Custom|SetBallOwner
  (params (Owner :type Actor%20Object%20Reference))
  ;[1 1 1] set ball owner
  (Variables|Default|SetPreviousOwner (Variables|Default|GetBallOwner))
  (bind _output_get (Variables|Default|SetBallOwner Owner))
  (CallFunction|BlockChangeOwnerfor 0.5)
  (Class|CharacterActionsInterfaceBP|BecameBallOwner(Message) _output_get self)
  (Default|CallOnOwnerChanged _output_get))

(event Custom|StartBounce
  (params (TargetPosition :type Vector) (Duration :type Float%20%28single-precision%29) (Distance :type Float%20%28single-precision%29) (MovementSpeed :type Float%20%28single-precision%29) (MovementDirection :type Vector) (StartHand :type ELeadHand%20Enum :default "NewEnumerator0") (BounceFinishHand :type ELeadHand%20Enum :default "NewEnumerator0") (MaxSpeed :type Float%20%28single-precision%29) (DedicatedToActor :type Actor%20Object%20Reference))
  ;[0.9516 0.7001 1] starters
  ;;[1 0.471 0] start bounce
  (Variables|Temp|SetBounceFinishHand BounceFinishHand)
  (bind _output_get (Utilities|CalculateMovementSpeedMultiplier MovementSpeed MaxSpeed))
  (bind _output_get_2 (Variables|Temp|SetMovementDirection MovementDirection))
  ;;;[1 1 1] predicted positions
  (Variables|Temp|SetPredictedEndPosition (+ TargetPosition (* _output_get_2 _output_get)))
  (Utilities|SetSpeedandDuration Duration Distance)
  (Utilities|IsValid DedicatedToActor
    (:Is%20Valid
      (bind _value (Class|SocketUtilsInterfaceBP|GetHandLocation(Message) DedicatedToActor StartHand))
      ;;;[1 1 1] discard temps
      (Variables|Temp|SetStartPosition _value)
      (Variables|Temp|SetTempAlpha 0.0))
    (:Is%20Not%20Valid
      ;;;[1 1 1] discard temps
      (Variables|Temp|SetStartPosition (Transformation|GetActorLocation))
      (Variables|Temp|SetTempAlpha 0.0))))

(event Custom|TryToPickBall
  (params (ByActor :type Actor%20Object%20Reference))
  ;[1 1 1] try to pick ball
  (bind _canpick (CallFunction|CanbePickedUp ByActor))
  (if _canpick
    (CallFunction|SetBallOwner ByActor)))

(event EventTick
  (params (DeltaSeconds :type Float%20%28single-precision%29))
  ;[1 1 1] tick
  (Networking|SwitchHasAuthority
    (:Authority
      (if (Utilities|Enum|NotEqual(Enum) (Variables|Default|GetCurrentActionType) "NewEnumerator6")
        (bind _interuptionactor (CallFunction|TryFindInteruptionPlayer))
        (Utilities|IsValid _interuptionactor
          (:Is%20Not%20Valid
            (CallFunction|MovementProccessing)))
        (else
          (Utilities|IsValid (Variables|Default|GetBallOwner)
            (:Is%20Valid
              (CallFunction|BallFollowing))
            (:Is%20Not%20Valid
              (CallFunction|ChecktoPickFreeBall))))))))

(event EventBeginPlay
  ;[0.08854 0.08854 0.08854] begin play
)

(fn ConstructionScript)

(fn FindChangeHandTargetPosition
  (bind _value (Class|SocketUtilsInterfaceBP|GetRootLocation(Message) (Variables|Default|GetBallOwner)))
  (return _value))

(fn GetPositionBallBouncefrom
  (bind _ballowner (Variables|Default|GetBallOwner))
  (bind _value (Class|SocketUtilsInterfaceBP|GetLeadHandLocation(Message) _ballowner))
  (bind _value_2 (Class|SocketUtilsInterfaceBP|GetRootLocation(Message) _ballowner))
  (return (Math|Vector|MakeVector (.X (Math|Vector|BreakVector _value)) (.Y (Math|Vector|BreakVector _value)) (.Z (Math|Vector|BreakVector _value_2)))))

(fn IsBusy
  (return (Utilities|Enum|NotEqual(Enum) (Variables|Default|GetCurrentActionType) "NewEnumerator6")))

(fn CurvePath
  (params (From :type Vector) (To :type Vector) (SegmentsCount :type Integer) (CurveMax :type Vector))
  (if (<= SegmentsCount 0)
    (Development|PrintString "Ball_BP:CurvePath: Invalid segments count")
    (else
      (LocalVariables|SetHeighestSegment (/ SegmentsCount 2))
      (for _index (range 0 SegmentsCount)
        (Utilities|Array|Add (LocalVariables|GetLocalPath) (+ (* CurveMax (Math|Float|MapRangeClamped (Math|Conversions|ToFloat(Integer) (- (LocalVariables|GetHeighestSegment) (Math|Integer|Absolute(Integer) (- (LocalVariables|GetHeighestSegment) _index)))) 0.0 (Math|Conversions|ToFloat(Integer) (LocalVariables|GetHeighestSegment)) 0.0 1.0)) (Math|Vector|Lerp(Vector) From To (* _index (/ (/ 1e+02 (Math|Conversions|ToFloat(Integer) SegmentsCount)) 1e+02))))))
      (return (LocalVariables|GetLocalPath)))))

(fn CalculateDistansePath
  (params (PathPoints :type Array%20of%20Vectors))
  (bind _returnvalue (Utilities|Array|Length PathPoints))
  (if (<= _returnvalue 1)
    (return (Math|Vector|VectorLength (Utilities|Array|Get(acopy) PathPoints)))
    (else
      (for (_array_element _array_index) PathPoints
        (if (== _array_index (- _returnvalue 1))
          (return (LocalVariables|GetLocalDistance))
          (else
            (LocalVariables|SetLocalDistance (+ (LocalVariables|GetLocalDistance) (Math|Vector|Distance(Vector) _array_element (Utilities|Array|Get(acopy) PathPoints (+ _array_index 1)))))))))))

(fn CanbePickedUp
  (params (ByActor :type Actor%20Object%20Reference))
  (Utilities|IsValid ByActor
    (:Is%20Valid
      (bind _value (Class|CharacterAttributesInterfaceBP|GetPickUpDistance(Message) ByActor))
      (if (>= _value (Transformation|GetDistanceTo ByActor self))
        (Utilities|IsValid (Variables|Default|GetBallOwner)
          (:Is%20Valid
            ;[1 1 1] for now return true for any requests
            (return true))
          (:Is%20Not%20Valid
            (return true)))
        (else
          (return false))))))

(fn GetNearestPlayer
  (bind _self self)
  (bind _allplayers (Variables|Default|GetAllPlayers))
  (for (_array_element _array_index) _allplayers
    (if (!= _array_element _self)
      (if (<= (LocalVariables|GetWithDistance) 0.0)
        (LocalVariables|SetWithDistance (Transformation|GetDistanceTo _array_element _self) :!label _label)
        (LocalVariables|SetNearestActorIndex _array_index)
        (elif (<= (Transformation|GetDistanceTo _array_element _self) (LocalVariables|GetWithDistance))
          (goto _label)))))
  (return (Utilities|Array|Get(acopy) _allplayers (LocalVariables|GetNearestActorIndex))))

(fn TryFindInteruptionPlayer
  (if (Variables|Default|GetBlockChangeOwner)
    _
    (else
      (for (_array_element _array_index) (Variables|Default|GetAllPlayers)
        (if (!= (Variables|Default|GetBallOwner) _array_element)
          (bind _array (Class|CharacterActionsInterfaceBP|GetInteruptStatesArray(Message) _array_element))
          (bind _value (Class|CharacterActionsInterfaceBP|GetCurrentState(Message) _array_element))
          (if (Utilities|Array|ContainsItem _array _value)
            (bind _value_2 (Class|CharacterAttributesInterfaceBP|GetStateLeadPoint(Message) _array_element _value))
            (bind _distance (Class|CharacterAttributesInterfaceBP|GetStateDistances(Message) _array_element _value))
            (if (>= _distance (Math|Vector|Distance(Vector) _value_2 (Transformation|GetActorLocation)))
              (if (or (<= (Math|Vector|Distance(Vector) _value_2 (Transformation|GetActorLocation)) (LocalVariables|GetLocalDistance)) (== (LocalVariables|GetLocalDistance) 0.0))
                (LocalVariables|SetLocalDistance (Math|Vector|Distance(Vector) _value_2 (Transformation|GetActorLocation)))
                (LocalVariables|SetLocalActorIndex _array_index)
                (LocalVariables|SetLocalState _value))))))
      (if (!= (LocalVariables|GetLocalActorIndex) -1)
        (return (Utilities|Array|Get(acopy) (Variables|Default|GetAllPlayers) (LocalVariables|GetLocalActorIndex)) (LocalVariables|GetLocalState))
        (else
          _))))
  (return 0 "NewEnumerator3"))