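; Holds a basketball character's attributes: skill values and height, with helpers to randomize and print them.
; Skills live in parallel key and value arrays, read by index lookup.
; Contests subtract the opponent's opposing skill, scaled by a multiplier, from this character's, logging outside packaged builds.
; GetContestOppositeFor has no wired logic, leaving the contest map lookup unused; the height-influence map does not enter the contest result.
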(fn GetContestMap
  (return (Utilities|Map|MakeMap "NewEnumerator0" "NewEnumerator3" "NewEnumerator1" "NewEnumerator3" "NewEnumerator2" "NewEnumerator3" "NewEnumerator9" "NewEnumerator10")))

(fn GetContestValuefor
  (params (Skill :type ECharacterSkills%20Enum :default "NewEnumerator0") (OtherAttributes :type Character%20Attributes%20BP%20Object%20Reference) (OtherAttributesMultiplier :type Float%20%28single-precision%29))
  (bind (_found _opposite) (Utilities|GetContestOppositefor Skill))
  (if _found
    (bind _value (CallFunction|GetSkillValue Skill))
    (bind _value_2 (CallFunction|GetSkillValue OtherAttributes _opposite))
    (if (Class|KismetSystemLibrary|IsPackagedforDistribution)
      _
      (else
        (Development|PrintString 0 (Utilities|String|Append "Contest between " (Utilities|String|Append (Utilities|String|EnumtoString Skill) ":" (Utilities|String|ToString(Float) _value)) " \\ " (Utilities|String|Append (Utilities|String|EnumtoString _opposite) ":" (Utilities|String|ToString(Float) (* _value_2 OtherAttributesMultiplier))) " with height " (Utilities|String|ToString(Float) (CallFunction|GetHeight)) "\\" (Utilities|String|ToString(Float) (CallFunction|GetHeight OtherAttributes)) " returns value = " (Class|KismetStringLibrary|ToUpper (Utilities|String|ToString(Float) (- _value (* _value_2 OtherAttributesMultiplier))))))))
    (return (- _value (* _value_2 OtherAttributesMultiplier)))
    (else
      (return 0.0))))

(fn GetSkillValue
  (params (Skill :type ECharacterSkills%20Enum :default "NewEnumerator0"))
  (bind _skillsdata (Variables|Default|GetSkillsData))
  (bind _returnvalue (Utilities|Array|FindItem _skillsdata Skill))
  (if (== _returnvalue -1)
    (return 0.0)
    (else
      (return (Utilities|Array|Get(acopy) (Variables|Default|GetSkillsValues) _returnvalue)))))

(fn GetHeightInfluenceMap
  (return (Utilities|Map|MakeMap "NewEnumerator0" 1.0 "NewEnumerator3" 1.0 "NewEnumerator10" -1.0 "NewEnumerator9" -0.5)))

(fn GetHeight
  (return (Variables|Default|GetHeight)))

(fn RandomizeValues
  (for _array_element (Variables|Default|GetSkillsValues)
    (Utilities|Array|Add (LocalVariables|GetLocalValues) (Math|Random|RandomFloatinRange 2e+01 1e+02)))
  (Variables|Default|SetSkillsValues (LocalVariables|GetLocalValues))
  (Variables|Default|SetHeight (Math|Random|RandomFloatinRange 1.5e+02 185.0)))

(fn DebugLogInfo
  (for (_array_element _array_index) (Variables|Default|GetSkillsData)
    (Development|PrintString 0 (Utilities|String|Append (Utilities|String|EnumtoString _array_element) " = " (Utilities|String|ToString(Float) (Utilities|Array|Get(acopy) (Variables|Default|GetSkillsValues) _array_index))) true true "(R=0.000000,G=0.660000,B=1.000000,A=1.000000)" 1e+01))
  (Development|PrintString 0 (Utilities|String|Append "Height" " = " (Utilities|String|ToString(Float) (Variables|Default|GetHeight))) true true "(R=0.000000,G=0.660000,B=1.000000,A=1.000000)" 1e+01)
  (Development|PrintString 0 "Your current attributes is:" true true "(R=0.000000,G=0.660000,B=1.000000,A=1.000000)" 1e+01))