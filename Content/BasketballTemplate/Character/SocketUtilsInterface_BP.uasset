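; Blueprint interface for the basketball template's characters that exposes queries for body socket positions.
; It declares getters for left, right, lead and specified hand locations, plus root, torso and overhead points.
; It also reports which hand leads and the distance between the root and a given hand.
; Function bodies return only zero or first-enum defaults, leaving the actual logic to implementing classes.
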(fn GetLeftHandLocation
  (return "0, 0, 0"))

(fn GetRightHandLocation
  (return "0, 0, 0"))

(fn GetRootLocation
  (return "0, 0, 0"))

(fn GetLeadHand
  (return "NewEnumerator0"))

(fn GetLeadHandLocation
  (return "0, 0, 0"))

(fn GetHandLocation
  (params (Hand :type ELeadHand%20Enum :default "NewEnumerator0"))
  (return "0, 0, 0"))

(fn GetDistanceBetweenRootandHand
  (params (Hand :type ELeadHand%20Enum :default "NewEnumerator0"))
  (return 0.0))

(fn GetTorsoLocation
  (return "0, 0, 0"))

(fn GetOverheadLocation
  (return "0, 0, 0"))