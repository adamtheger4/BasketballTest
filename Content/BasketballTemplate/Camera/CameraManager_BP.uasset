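; Basketball template camera actor that follows the first player's pawn and can flip to view the court from the opposite direction.
; Construction applies boom and camera settings; BeginPlay waits a second, saves its start position, then blends the view to itself.
; ChangeCamera compares facing and target side to start a 180-degree boom yaw flip, interpolated on Tick.
; Tick also repositions the actor behind the pawn, scaling sideways Y movement against scene width.
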(event Custom|ApplySettings
  (bind _camera (Variables|Default|GetCamera))
  ;[1 1 1] apply settings
  (Variables|/Script/Engine.SpringArmComponent|SetTargetArmLength (Variables|Default|GetCameraBoom) (Variables|Settings|GetArmDistance))
  (Transformation|SetRelativeLocation _camera (Math|Vector|MakeVector 0.0 0.0 (Variables|Settings|GetHeight)) false true)
  (Transformation|SetRelativeRotation _camera (Math|Rotator|MakeRotator 0.0 (Variables|Settings|GetCameraPitch) 0.0) false true))

(event Custom|FollowOwnedPawn
  (bind _returnvalue (Game|GetPlayerController 0))
  (bind _camera (Variables|Default|GetCamera))
  (bind _armdistance (Variables|Settings|GetArmDistance))
  (bind _returnvalue_2 (Pawn|GetControlledPawn _returnvalue))
  (bind _returnvalue_3 (Math|Vector|GetForwardVector _camera))
  (bind _returnvalue_4 (Transformation|GetActorLocation _returnvalue_2))
  (bind _returnvalue_5 (* _returnvalue_3 _armdistance))
  (bind _returnvalue_6 (* _returnvalue_5 -1.0))
  (bind _returnvalue_7 (+ _returnvalue_4 _returnvalue_6))
  (bind (_x _y _z) (Math|Vector|BreakVector _returnvalue_7))
  ;[1 1 1] follow owned pawn
  (Utilities|IsValid _returnvalue_2
    (:Is%20Valid
      (Transformation|SetActorLocation (Math|Vector|MakeVector _x (Math|Float|Lerp 0.0 (Variables|AdditionalSettings|GetCameraMovementMaxY) (/ (.Y (Math|Vector|BreakVector _returnvalue_4)) (Variables|AdditionalSettings|GetSceneMaxY))) _z) false true))))

(event Custom|ChangeCamera
  (params (ToTarget :type Vector) (TargetForwardVector :type Vector) (BlendSpeed :type Float%20%28single-precision%29))
  (bind _returnvalue (* 2.0 BlendSpeed))
  ;[1 1 1] change camera
  (bind _value (CallFunction|AlreadyLookon TargetForwardVector))
  (if (not _value)
    (if (>= (.x (Math|Vector|GetUnitDirection(Vector) ToTarget (Variables|AdditionalSettings|GetStartPosition))) 0.0)
      (CallFunction|FlipArmLenghtandCameraRotation 0.0 1.8e+02 _returnvalue)
      (else
        (CallFunction|FlipArmLenghtandCameraRotation 1.8e+02 0.0 _returnvalue)))))

(event Custom|FlipArmLenghtAndCameraRotation
  (params (FromRotationZ :type Float%20%28single-precision%29) (TargetRotationZ :type Float%20%28single-precision%29) (BlendPerSec :type Float%20%28single-precision%29))
  ;[1 1 1] flip arm lenght and rot
  (Variables|Temp|SetFromRotationZ FromRotationZ)
  (Variables|Temp|SetTargetRotationZ TargetRotationZ)
  (Variables|Temp|SetBlendPerSec BlendPerSec)
  (Variables|Temp|SetTempAlpha 0.0)
  (Variables|Temp|SetChangeCameraPosition true))

(event Custom|ProccedChangingCamera
  (bind _cameraboom (Variables|Default|GetCameraBoom))
  (bind _relativerotation (Variables|/Script/Engine.SceneComponent|GetRelativeRotation _cameraboom))
  ;[1 1 1] procced changing camera
  (if (Variables|Temp|GetChangeCameraPosition)
    (bind _output_get (Variables|Temp|SetTempAlpha (Math|Float|Clamp(Float) (+ (Variables|Temp|GetTempAlpha) (* (Variables|Temp|GetBlendPerSec) (Utilities|Time|GetWorldDeltaSeconds))))))
    (if (>= _output_get 1.0)
      (Variables|Temp|SetChangeCameraPosition false))
    (Transformation|SetRelativeRotation _cameraboom (Math|Rotator|MakeRotator (.roll _relativerotation) (.pitch _relativerotation) (Math|Float|Lerp (Variables|Temp|GetFromRotationZ) (Variables|Temp|GetTargetRotationZ) (Variables|Temp|GetTempAlpha))) false false)))

(event EventTick
  (params (DeltaSeconds :type Float%20%28single-precision%29))
  ;[1 1 1] tick
  (CallFunction|ProccedChangingCamera)
  (CallFunction|FollowOwnedPawn))

(event EventBeginPlay
  ;[1 1 1] begin play
  ;;[1 1 1] temp, it create earlier than camera on character so need to delay
  (Utilities|FlowControl|Delay 1.0)
  (Variables|AdditionalSettings|SetStartPosition (Transformation|GetActorLocation))
  (Game|Player|SetViewTargetwithBlend (Game|GetPlayerController 0) self 2.0 "VTBlend_Cubic" 0.0 false))

(fn ConstructionScript
  (CallFunction|ApplySettings))

(fn AlreadyLookon
  (params (TargetForwardVector :type Vector))
  (bind _x (Math|Vector|BreakVector TargetForwardVector))
  (if (> (.X (Math|Vector|BreakVector (Math|Vector|GetForwardVector (Variables|Default|GetCamera)))) 0.0)
    (return (< _x 0.0))
    (else
      (return (> _x 0.0)))))