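; Basketball court in-bounds zone that fires OnOutOfBounds on the server when a pawn leaves its Box.
; Helpers derive court corners from the Box bounds and generate random positions around an origin or in front of a hoop.
; Random streams are seeded by current millisecond plus an index, with X and Y sharing each seed.
; GetNearestOutOfBoundsPosition normalizes a point within the bounds to choose an end line or sideline exit spot.
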(event OnComponentEndOverlap(Box)
  (params (OverlappedComponent :type Primitive%20Component%20Object%20Reference) (OtherActor :type Actor%20Object%20Reference) (OtherComp :type Primitive%20Component%20Object%20Reference) (OtherBodyIndex :type Integer))
  (Networking|SwitchHasAuthority
    (:Authority
      (bind _aspawn (Utilities|Casting|CastToPawn OtherActor))
      (Default|CallOnOutOfBounds _aspawn))))

(event EventBeginPlay)

(event Collision|EventActorBeginOverlap
  (params (OtherActor :type Actor%20Object%20Reference)))

(event EventTick
  (params (DeltaSeconds :type Float%20%28single-precision%29)))

(fn ConstructionScript)

(fn GetRandomLocationsInbound
  (params (Origin :type Vector) (InRadius :type Float%20%28single-precision%29) (Count :type Integer))
  (bind (_downleftlocation _uprightlocation) (CallFunction|GetBounds))
  (bind _locations (CallFunction|GetRandomLocationsInboundinRange Origin InRadius Count (Math|Vector2D|MakeVector2D (.X (Math|Vector|BreakVector _uprightlocation)) (.Y (Math|Vector|BreakVector _uprightlocation))) (Math|Vector2D|MakeVector2D (.X (Math|Vector|BreakVector _downleftlocation)) (.Y (Math|Vector|BreakVector _downleftlocation)))))
  (return _locations))

(fn GetBounds
  (bind _box (Variables|Default|GetBox))
  (bind (_origin _boxextent) (Collision|GetComponentBounds _box))
  (bind (_x _y) (Math|Vector|BreakVector _boxextent))
  (bind (_x_2 _y_2) (Math|Vector|BreakVector _origin))
  (bind _returnvalue (Math|Vector|MakeVector _x _y 0.0))
  (bind _returnvalue_2 (Math|Vector|MakeVector _x_2 _y_2 0.0))
  (bind _returnvalue_3 (- _returnvalue_2 _returnvalue))
  (bind _returnvalue_4 (+ _returnvalue_2 _returnvalue))
  (return (Math|Vector|MakeVector (.x _returnvalue_4) (.y _returnvalue_4) 2e+01) (Math|Vector|MakeVector (.x _returnvalue_3) (.y _returnvalue_3) 2e+01)))

(fn GetRandomLocationsInboundinRange
  (params (Origin :type Vector) (InRadius :type Float%20%28single-precision%29) (Count :type Integer) (RangeBoundsFirst :type Vector%202D%20Structure) (RangeBoundsSecond :type Vector%202D%20Structure))
  (bind (_x _y) (Math|Vector2D|BreakVector2D RangeBoundsFirst))
  (bind (_x_2 _y_2) (Math|Vector2D|BreakVector2D RangeBoundsSecond))
  (bind _returnvalue (Math|DateTime|UTCNow))
  (bind _locallocation (LocalVariables|GetLocalLocation))
  (bind _returnvalue_2 (Utilities|Array|Length _locallocation))
  (bind _returnvalue_3 (Math|DateTime|GetMillisecond _returnvalue))
  (bind _returnvalue_4 (+ _returnvalue_3 _returnvalue_2))
  (bind _returnvalue_5 (Math|Random|MakeRandomStream _returnvalue_4))
  (for _index (range 0 (- Count 1))
    (Utilities|Array|Add (LocalVariables|GetLocalLocation) (+ (* (Math|Vector|GetUnitDirection(Vector) Origin (Math|Vector|MakeVector (Math|Random|RandomFloatinRangefromStream _x_2 _x _returnvalue_5) (Math|Random|RandomFloatinRangefromStream _y_2 _y _returnvalue_5) 2e+01)) InRadius) Origin)))
  (return (LocalVariables|GetLocalLocation)))

(fn GetRandomLocationsInboundinAngle
  (params (FromPosition :type Vector) (ToPosition :type Vector) (InRadius :type Float%20%28single-precision%29) (Count :type Integer) (RangeBoundsFirst :type Vector%202D%20Structure) (RangeBoundsSecond :type Vector%202D%20Structure))
  (bind (_x _y) (Math|Vector2D|BreakVector2D RangeBoundsFirst))
  (bind (_x_2 _y_2) (Math|Vector2D|BreakVector2D RangeBoundsSecond))
  (bind _returnvalue (Math|DateTime|UTCNow))
  (bind _locallocation (LocalVariables|GetLocalLocation))
  (bind _returnvalue_2 (Utilities|Array|Length _locallocation))
  (bind _returnvalue_3 (Math|DateTime|GetMillisecond _returnvalue))
  (bind _returnvalue_4 (+ _returnvalue_3 _returnvalue_2))
  (bind _returnvalue_5 (Math|Random|MakeRandomStream _returnvalue_4))
  (for _index (range 0 (- Count 1))
    (Utilities|Array|Add (LocalVariables|GetLocalLocation) (+ (* (Math|Vector|GetUnitDirection(Vector) FromPosition (Math|Vector|MakeVector (Math|Random|RandomFloatinRangefromStream _x_2 _x _returnvalue_5) (Math|Random|RandomFloatinRangefromStream _y_2 _y _returnvalue_5) 2e+01)) InRadius) FromPosition)))
  (return (LocalVariables|GetLocalLocation)))

(fn GetCenterAttackPositionto
  (params (HoopLocation :type Vector) (OnDistance :type Float%20%28single-precision%29))
  (return (* (Math|Vector|GetUnitDirection(Vector) HoopLocation (Transformation|GetActorLocation)) OnDistance)))

(fn GetRandomLocationsfromHoopinBounds
  (params (HoopPosition :type Vector) (HoopForwardDirection :type Vector) (Distance :type Float%20%28single-precision%29) (Count :type Integer) (XRange :type Float%20%28single-precision%29) (YRange :type Float%20%28single-precision%29))
  (for _index (range 0 (- Count 1))
    (bind _returnvalue (CallFunction|GetRandomLocationinBounds (Utilities|Array|Length (LocalVariables|GetLocalLocation)) (Math|Vector2D|MakeVector2D XRange YRange) (Math|Vector2D|MakeVector2D (* XRange -1.0) (* YRange -1.0))))
    (Utilities|Array|Add (LocalVariables|GetLocalLocation) (Math|Vector|MakeVector (.x (+ _returnvalue (+ HoopPosition (* HoopForwardDirection Distance)))) (.y (+ _returnvalue (+ HoopPosition (* HoopForwardDirection Distance)))) 2e+01)))
  (return (LocalVariables|GetLocalLocation)))

(fn GetRandomLocationinBounds
  (params (AddToRandom :type Integer) (BoundsFirst :type Vector%202D%20Structure) (BoundsSecond :type Vector%202D%20Structure))
  (bind (_x _y) (Math|Vector2D|BreakVector2D BoundsFirst))
  (bind (_x_2 _y_2) (Math|Vector2D|BreakVector2D BoundsSecond))
  (bind _returnvalue (Math|DateTime|UTCNow))
  (bind _returnvalue_2 (Math|DateTime|GetMillisecond _returnvalue))
  (bind _returnvalue_3 (+ _returnvalue_2 AddToRandom))
  (bind _returnvalue_4 (Math|Random|MakeRandomStream _returnvalue_3))
  (return (Math|Vector|MakeVector (Math|Random|RandomFloatinRangefromStream _x_2 _x _returnvalue_4) (Math|Random|RandomFloatinRangefromStream _y_2 _y _returnvalue_4) 2e+01)))

(fn GetNearestOutOfBoundsPosition
  (params (InboundPosition :type Vector))
  (bind (_x _y) (Math|Vector|BreakVector InboundPosition))
  ;[1 1 1] transform position to 0...1 range
  (bind (_downleftlocation _uprightlocation) (CallFunction|GetBounds))
  (if (or (>= (Math|Float|NormalizetoRange _x (.X (Math|Vector|BreakVector _uprightlocation)) (.X (Math|Vector|BreakVector _downleftlocation))) 0.9) (<= (Math|Float|NormalizetoRange _x (.X (Math|Vector|BreakVector _uprightlocation)) (.X (Math|Vector|BreakVector _downleftlocation))) 0.1))
    (return (Math|Vector|MakeVector (Math|Float|SelectFloat (Math|Float|Lerp _x (.X (Math|Vector|BreakVector _downleftlocation)) 1.05) (Math|Float|Lerp (.X (Math|Vector|BreakVector _downleftlocation)) _x 1.05) (>= (Math|Float|NormalizetoRange _x (.X (Math|Vector|BreakVector _uprightlocation)) (.X (Math|Vector|BreakVector _downleftlocation))) 0.5)) (Math|Float|Lerp (.Y (Math|Vector|BreakVector _uprightlocation)) (.Y (Math|Vector|BreakVector _downleftlocation)) (Math|Float|NormalizetoRange _y (.Y (Math|Vector|BreakVector _uprightlocation)) (.Y (Math|Vector|BreakVector _downleftlocation)))) (.Z (Math|Vector|BreakVector InboundPosition))))
    (else
      (return (Math|Vector|MakeVector (Math|Float|Lerp (.X (Math|Vector|BreakVector _uprightlocation)) (.X (Math|Vector|BreakVector _downleftlocation)) (Math|Float|NormalizetoRange _x (.X (Math|Vector|BreakVector _uprightlocation)) (.X (Math|Vector|BreakVector _downleftlocation)))) (Math|Float|SelectFloat (Math|Float|Lerp (.Y (Math|Vector|BreakVector _uprightlocation)) (.Y (Math|Vector|BreakVector _downleftlocation)) 1.05) (Math|Float|Lerp (.Y (Math|Vector|BreakVector _downleftlocation)) (.Y (Math|Vector|BreakVector _uprightlocation)) 1.05) (>= (Math|Float|NormalizetoRange _y (.Y (Math|Vector|BreakVector _uprightlocation)) (.Y (Math|Vector|BreakVector _downleftlocation))) 0.5)) (.Z (Math|Vector|BreakVector InboundPosition)))))))

(fn GetBoundsSize
  (bind _box (Variables|Default|GetBox))
  (bind _boxextent (Collision|GetComponentBounds _box))
  (bind (_x _y) (Math|Vector|BreakVector _boxextent))
  (return _x _y))