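; Basketball hoop Blueprint that decides whether a player's shot scores and supplies the path for that outcome.
; GetPathDataFor rolls against the player's success chance, then returns the success spline or one of two random failure splines, with a success index (-1 on failure).
; CalculatePathBy converts the chosen spline's points to world-space locations.
; GetInputPathPoint exposes the success path's first point.
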(fn ConstructionScript)

(fn GetSuccessPath
  (CallFunction|CalculatePathby (Variables|Default|GetSuccessPath1))
  (return (Variables|Default|GetCalculatedPreviousPath)))

(fn CalculatePathby
  (params (Spline :type Spline%20Component%20Object%20Reference))
  (Utilities|Array|Clear (Variables|Default|GetCalculatedPreviousPath))
  (for _index (range 0 (- (Spline|GetNumberOfSplinePoints Spline) 1))
    (Utilities|Array|Add (Variables|Default|GetCalculatedPreviousPath) (Spline|GetLocationatSplinePoint Spline _index "World"))))

(fn GetInputPathPoint
  (CallFunction|CalculatePathby (Variables|Default|GetSuccessPath1))
  (return (Utilities|Array|Get(acopy) (Variables|Default|GetCalculatedPreviousPath))))

(fn GetPathDatafor
  (params (Player :type Actor%20Object%20Reference))
  (bind _value (Class|CharacterAttributesInterfaceBP|GetChancetoSuccessShot(Message) Player))
  (if (Math|Random|RandomBoolwithWeight _value)
    (Development|PrintString "Success shot")
    (bind _path (CallFunction|GetSuccessPath))
    (return _path 2)
    (else
      (Development|PrintString "Failure shot")
      (bind _path_2 (CallFunction|GetFailurePath))
      (return _path_2 -1))))

(fn GetFailurePath
  (CallFunction|CalculatePathby (select (Math|Random|RandomBool) (Variables|Default|GetFailurePath2) (Variables|Default|GetFailurePath1)))
  (return (Variables|Default|GetCalculatedPreviousPath)))

(fn GetPathDatafor
  (params (Player :type Actor%20Object%20Reference))
  (bind (_path _successindex) (CallFunction|GetPathDatafor Player))
  (return _path _successindex))