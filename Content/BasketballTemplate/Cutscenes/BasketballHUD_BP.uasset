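; Basketball HUD that shows the clock and both team scores, plus toggleable notification widgets and a plug widget.
; StartNotificationSystem stores the game state and creates the bottom-right time/score widget, which Tick refreshes while visible, adding a tenths digit in the final seconds.
; Notification widgets are looked up by type through parallel enum, class and reference arrays, and created on demand before being added to or removed from the viewport.
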(event Custom|HidePlugWidget
  ;[1 1 1] plug widget
  (Utilities|IsValid (Variables|Default|GetViewPlug)
    (:Is%20Valid
      (Widget|RemovefromParent (Variables|Default|GetViewPlug)))))

(event Custom|ShowPlugWidget
  ;[1 1 1] plug widget
  (Utilities|IsValid (Variables|Default|GetViewPlug)
    (:Is%20Valid
      _)
    (:Is%20Not%20Valid
      (bind _returnvalue (UserInterface|CreateWidget "/Game/BasketballTemplate/Cutscenes/ViewPlugWIdget_BP.ViewPlugWIdget_BP_C" (Game|GetPlayerController 0)))
      (Variables|Default|SetViewPlug _returnvalue)))
  (UserInterface|Viewport|AddtoViewport (Variables|Default|GetViewPlug) 0))

(event Custom|StartNotificationSystem
  (params (CurrentGameState :type Game%20Settings%20Actor%20BP%20Object%20Reference))
  ;[1 1 1] notification system
  (Variables|Default|SetGameState CurrentGameState)
  (bind _returnvalue (UserInterface|CreateWidget "/Game/BasketballTemplate/Cutscenes/TimeScoreWIdget_BP.TimeScoreWIdget_BP_C" (Game|GetPlayerController 0)))
  (bind _output_get (Variables|Default|SetTimeScore _returnvalue))
  (Class|UserWidget|SetDesiredSizeinViewport _output_get "(X=400.000000,Y=200.000000)")
  (Class|UserWidget|SetAnchorsinViewport _returnvalue (Utilities|Struct|MakeAnchors "(X=1.000000,Y=1.000000)" "(X=1.000000,Y=1.000000)"))
  (Class|UserWidget|SetAlignmentinViewport _output_get "(X=1.000000,Y=1.000000)")
  (UserInterface|Viewport|AddtoViewport _output_get 0))

(event Custom|SetHiddenNotificationSystem
  (params (Hidden :type Boolean))
  (bind _timescore (Variables|Default|GetTimeScore))
  ;[1 1 1] notification system
  (Utilities|IsValid _timescore
    (:Is%20Valid
      (Widget|SetVisibility _timescore (select Hidden "Hidden" "Visible")))))

(event Custom|UpdateNotificationSystem
  (bind _returnvalue (Math|DateTime|UTCNow))
  (bind _timescore (Variables|Default|GetTimeScore))
  (bind _gamestate (Variables|Default|GetGameState))
  (bind _gamestate_2 (Variables|Default|GetGameState))
  (bind _clocktotime (Variables|/Game/BasketballTemplate/GameSettingsActor_BP.GameSettingsActor_BP_C|GetClockToTime _gamestate_2))
  (bind _returnvalue_2 (- _clocktotime _returnvalue))
  (bind _returnvalue_3 (Math|Timespan|GetSeconds _returnvalue_2))
  ;[1 1 1] update notification system
  (Utilities|IsValid _timescore
    (:Is%20Valid
      (if (Widget|IsVisible _timescore)
        (Utilities|IsValid (Variables|Default|GetGameState)
          (:Is%20Valid
            (Default|SetTime (Variables|Default|GetTimeScore) (select (<= _returnvalue_3 4) (Utilities|Text|FormatText "{s}.{ms}" _returnvalue_3 (Utilities|String|Left (Utilities|String|ToString(Integer) (Class|KismetMathLibrary|GetMilliseconds _returnvalue_2)) 1)) (Utilities|Text|ToText(Integer) _returnvalue_3)))
            (Default|SetScore (Variables|Default|GetTimeScore) (Utilities|Text|ToText(Integer) (Variables|/Game/BasketballTemplate/GameSettingsActor_BP.GameSettingsActor_BP_C|GetTeam1Score _gamestate)) (Utilities|Text|ToText(Integer) (Variables|/Game/BasketballTemplate/GameSettingsActor_BP.GameSettingsActor_BP_C|GetTeam2Score _gamestate)))))))))

(event Custom|SetNotificationWidgetState
  (params (Type :type ENotificationType%20Enum :default "NewEnumerator0") (State :type Boolean))
  ;[1 1 1] set notification widget state
  (bind _widget (CallFunction|GetNotificationWidget Type))
  (if State
    (Class|UserWidget|SetDesiredSizeinViewport _widget "(X=300.000000,Y=200.000000)")
    (Class|UserWidget|SetAnchorsinViewport _widget (Utilities|Struct|MakeAnchors "(X=1.000000,Y=1.000000)" "(X=1.000000,Y=1.000000)"))
    (Class|UserWidget|SetAlignmentinViewport _widget "(X=1.000000,Y=2.000000)")
    (UserInterface|Viewport|AddtoViewport _widget 0)
    (else
      (Widget|RemovefromParent _widget))))

(event EventBeginPlay)

(event EventTick
  (params (DeltaSeconds :type Float%20%28single-precision%29))
  ;[1 1 1] tick
  (CallFunction|UpdateNotificationSystem))

(fn ConstructionScript)

(fn GetNotificationWidget
  (params (ItemToFind :type ENotificationType%20Enum%20%28by%20ref%29 :default "NewEnumerator0"))
  (bind _notificationenumindex (Variables|Notififcation|GetNotificationEnumIndex))
  (bind _returnvalue (Utilities|Array|FindItem _notificationenumindex ItemToFind))
  (if (!= _returnvalue -1)
    (Utilities|IsValid (Utilities|Array|Get(acopy) (Variables|Notififcation|GetNotificationWidgetRef) _returnvalue)
      (:Is%20Valid
        _)
      (:Is%20Not%20Valid
        (bind _returnvalue_2 (UserInterface|CreateWidget (Utilities|Array|Get(acopy) (Variables|Notififcation|GetNotificationWidgetClass) _returnvalue) (Game|GetPlayerController 0)))
        (Utilities|Array|Insert (Variables|Notififcation|GetNotificationWidgetRef) _returnvalue_2 _returnvalue)))
    (return (Utilities|Array|Get(acopy) (Variables|Notififcation|GetNotificationWidgetRef) _returnvalue))))