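; GameSettingsActor_BP holds basketball match state: the game clock, two team scores and the active hoop.
; The clock stores a UTC end time and runs a one-shot timer that broadcasts OnClockIsOver on expiry.
; Hoop switching validates the index and broadcasts changes, with a RepNotify on ActiveHoop repeating the broadcast for replication.
; AddTeamScore adds points to the given team and returns its new total.
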(event Custom|ChangeActiveHoop
  (params (SelectHoopAt :type Integer))
  (bind _hoops (Variables|Default|GetHoops))
  (bind _output (Utilities|Array|Get(acopy) _hoops SelectHoopAt))
  ;[1 1 1] change active hoop
  (if (Math|Integer|InRange(Integer) SelectHoopAt 0 (Utilities|Array|Length (Variables|Default|GetHoops)) true false)
    (if (!= (Variables|Default|GetActiveHoop) _output)
      (Variables|Default|SetActiveHoop _output)
      (Default|CallOnActiveHoopChanged (Variables|Default|GetActiveHoop)))))

(event Custom|SetClockTimerFor
  (params (Seconds :type Integer))
  ;[1 1 1] set clock time to
  (Variables|Default|SetClockToTime (+ (Math|DateTime|UTCNow) (Math|Timespan|MakeTimespan 0 0 0 Seconds)))
  (Utilities|Time|ClearandInvalidateTimerbyHandle (Variables|Default|GetClockTimerHandle))
  (bind _returnvalue (Utilities|Time|SetTimerbyEvent (delegate Custom|ClockIsOver) (Math|Conversions|ToFloat(Integer) Seconds)))
  (Variables|Default|SetClockTimerHandle _returnvalue))

(event Custom|ClockIsOver
  ;[1 1 1] set clock time to
  (Default|CallOnClockIsOver))

(fn ConstructionScript)

(fn OnRepActiveHoop
  (Default|CallOnActiveHoopChanged (Variables|Default|GetActiveHoop)))

(fn AddTeamScore
  (params (TeamId :type Integer) (Value :type Integer))
  (switch int TeamId
    (:0
      (bind _output_get (Variables|Default|SetTeam1Score (+ (Variables|Default|GetTeam1Score) Value)))
      (return _output_get))
    (:1
      (bind _output_get_2 (Variables|Default|SetTeam2Score (+ Value (Variables|Default|GetTeam2Score))))
      (return _output_get_2))))