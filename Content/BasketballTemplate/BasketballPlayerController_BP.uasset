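; Basketball player controller that runs the out-of-bounds inbound flow, the local camera and HUD notifications, and exposes ball, hoop and team getters from GameSettings.
; Out-of-bounds blocks pawn input until a pass press resumes play, with movement constrained and forwarded on the X axis after a basket.
; Keyed input blockers stack and replicate via RepNotify.
; Once GameSettings is valid, active hoop changes retarget the pawn and, locally, the spawned camera manager.
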(event Custom|OnChangedServerTargetHoop
  (params (NewActiveHoop :type Actor%20Object%20Reference))
  ;[1 1 1] temp: need to set target hoop to the server-side pawn
  (Class|CharacterActionsInterfaceBP|SetTargetHoop(Message) (Pawn|GetControlledPawn) NewActiveHoop))

(event Custom|OnChangedTargetHoop
  (params (NewActiveHoop :type Actor%20Object%20Reference))
  (bind _gamesettings (Variables|Default|GetGameSettings))
  (bind _activehoop (Variables|/Game/BasketballTemplate/GameSettingsActor_BP.GameSettingsActor_BP_C|GetActiveHoop _gamesettings))
  ;[1 1 1] on change target hoop
  (Default|ChangeCamera (Variables|Default|GetCameraManager) (Transformation|GetActorLocation _activehoop) (Transformation|GetActorForwardVector _activehoop) 1.0)
  (Class|CharacterActionsInterfaceBP|SetTargetHoop(Message) (Pawn|GetControlledPawn) _activehoop))

(event Custom|SetNotificationWidgetState
  (params (Type :type ENotificationType%20Enum :default "NewEnumerator0") (State :type Boolean))
  ;[1 1 1] notification system
  ;;[1 1 1] SetNotificationWidgetState
  (bind _asbasketball_hud_bp (Utilities|Casting|CastToBasketballHUD_BP (HUD|GetHUD)))
  (Default|SetNotificationWidgetState _asbasketball_hud_bp Type State))

(event Custom|RecheckInputPossibility
  ;[1 1 1] recheck inputs possibility
  (if (> (Utilities|Array|Length (Variables|Default|GetInputKeysBlocker)) 0)
    (Input|DisableInput (Pawn|GetControlledPawn) self)
    (else
      (Input|EnableInput (Pawn|GetControlledPawn) self))))

(event Custom|SetHiddenNotificationSystem
  (params (Hidden :type Boolean))
  ;[1 1 1] notification system
  ;;[1 1 1] set hidden notification system
  (bind _asbasketball_hud_bp (Utilities|Casting|CastToBasketballHUD_BP (HUD|GetHUD)))
  (Default|SetHiddenNotificationSystem _asbasketball_hud_bp Hidden))

(event Custom|ServerHideViewPlugAnimation
  ;[1 1 1] plug view animation
  (CallFunction|EnableInputwith 1)
  (CallFunction|ClientSetViewPlugAnimation false))

(event Custom|ClientSetViewPlugAnimation
  (params (Enabled :type Boolean))
  ;[1 1 1] plug view animation
  (bind _asbasketball_hud_bp (Utilities|Casting|CastToBasketballHUD_BP (HUD|GetHUD)))
  (if Enabled
    (Default|ShowPlugWidget _asbasketball_hud_bp)
    (else
      (Default|HidePlugWidget _asbasketball_hud_bp))))

(event Custom|DisableInputWith
  (params (InputKey :type Byte))
  ;[1 1 1] inputs: Its done for not activate inputs while itf disactivated by someone else
  (Utilities|Array|Add (Variables|Default|GetInputKeysBlocker) InputKey)
  (CallFunction|RecheckInputPossibility))

(event Custom|ServerShowViewPlugAnimation
  ;[1 1 1] plug view animation
  (CallFunction|DisableInputwith 1)
  (CallFunction|ClientSetViewPlugAnimation true))

(event Custom|EnableInputWith
  (params (InputKey :type Byte))
  ;[1 1 1] inputs: Its done for not activate inputs while itf disactivated by someone else
  (Utilities|Array|RemoveItem (Variables|Default|GetInputKeysBlocker) InputKey)
  (CallFunction|RecheckInputPossibility))

(event Custom|SpawnClientCameraManger
  ;[1 1 1] spawn client camera manager
  (bind _returnvalue (Game|SpawnActorfromClass "/Game/BasketballTemplate/Camera/CameraManager_BP.CameraManager_BP_C" (Math|Transform|MakeTransform "-972.000000, 0, 0") "Undefined" 0 self))
  (Variables|Default|SetCameraManager _returnvalue))

(event Custom|ProccedOutOfBounds
  (params (AfterBasket :type Boolean) (PassToTeammate :type Boolean))
  ;[1 1 1] out of bounds
  (Variables|Default|SetOutOfBoundPassToTeammate PassToTeammate)
  (Variables|Default|SetOutOfBounds true)
  (Variables|Default|SetOutOfBoundAfterBasket AfterBasket)
  (Class|CharacterActionsInterfaceBP|ProccedOutOfBounds(Message) (Pawn|GetControlledPawn))
  (CallFunction|DisableInputwith 2)
  ;;[1 1 1] for listen-server client while we are after basket (client do it by rep-notify)
  (if (Variables|Default|GetOutOfBoundAfterBasket)
    (Class|CharacterActionsInterfaceBP|SetMovementConstrain(Message) (Pawn|GetControlledPawn) true "X")))

(event Custom|ApplyOutOfBounds
  ;[1 1 1] out of bounds
  (Variables|Default|SetOutOfBounds false)
  (Class|CharacterActionsInterfaceBP|ApplyOutOfBounds(Message) (Pawn|GetControlledPawn) (Variables|Default|GetOutOfBoundPassToTeammate))
  (CallFunction|EnableInputwith 2)
  ;;[1 1 1] for listen-server client while we are after basket (client do it by rep-notify)
  (if (Variables|Default|GetOutOfBoundAfterBasket)
    (Variables|Default|SetOutOfBoundAfterBasket false)
    (Class|CharacterActionsInterfaceBP|SetMovementConstrain(Message) (Pawn|GetControlledPawn) false "Custom")))

(event Custom|StartNotificationSystem
  ;[1 1 1] notification system
  ;;[1 1 1] start notification system
  (bind _asbasketball_hud_bp (Utilities|Casting|CastToBasketballHUD_BP (HUD|GetHUD)))
  (Default|StartNotificationSystem _asbasketball_hud_bp (Variables|Default|GetGameSettings)))

(event EventBeginPlay
  (bind _gamesettings (Variables|Default|GetGameSettings))
  (bind _gamesettings_2 (Variables|Default|GetGameSettings))
  (bind _activehoop (Variables|/Game/BasketballTemplate/GameSettingsActor_BP.GameSettingsActor_BP_C|GetActiveHoop _gamesettings_2))
  ;[1 1 1] begin play
  (if (Pawn|IsLocalPlayerController)
    (CallFunction|SpawnClientCameraManger)
    (Utilities|IsValid _gamesettings_2 :!label _label
      (:Is%20Valid
        (CallFunction|StartNotificationSystem)
        (EventDispatchers|BindEventtoOnActiveHoopChanged _gamesettings_2 (delegate Custom|OnChangedTargetHoop))
        (Utilities|IsValid _activehoop
          (:Is%20Valid
            (CallFunction|OnChangedTargetHoop _activehoop))))
      (:Is%20Not%20Valid
        (Utilities|FlowControl|Delay 0.0)
        (goto _label)))
    (else
      ;[1 1 1] temp: need to set target hoop to the server-side pawn
      (Utilities|IsValid _gamesettings :!label _label_2
        (:Is%20Valid
          (EventDispatchers|BindEventtoOnActiveHoopChanged _gamesettings (delegate Custom|OnChangedServerTargetHoop)))
        (:Is%20Not%20Valid
          (Utilities|FlowControl|Delay 0.0)
          (goto _label_2))))))

(event Input|ActionEvents|InputActionPassRegular
  (params (Key :type Key%20Structure :default "None"))
  ;[1 1 1] out of bounds
  (:Pressed
    (if (Variables|Default|GetOutOfBounds)
      (CallFunction|ApplyOutOfBounds))))

(event Input|ActionEvents|InputActionPassBounce
  (params (Key :type Key%20Structure :default "None"))
  ;[1 1 1] out of bounds
  (:Pressed
    (if (Variables|Default|GetOutOfBounds)
      (CallFunction|ApplyOutOfBounds))))

(event Input|AxisEvents|InputAxisMoveForward
  (params (AxisValue :type Float%20%28single-precision%29))
  ;[1 1 1] out of bounds
  (if (Variables|Default|GetOutOfBounds)
    (if (Variables|Default|GetOutOfBoundAfterBasket)
      (Class|CharacterActionsInterfaceBP|MoveForward(Message) (Pawn|GetControlledPawn) AxisValue))))

(event Input|AxisEvents|InputAxisMoveRight
  (params (AxisValue :type Float%20%28single-precision%29))
  ;[1 1 1] out of bounds
  (if (Variables|Default|GetOutOfBounds)
    (if (Variables|Default|GetOutOfBoundAfterBasket)
      (Class|CharacterActionsInterfaceBP|MoveRight(Message) (Pawn|GetControlledPawn) AxisValue))))

(event Input|KeyboardEvents|NumPadOne
  (params (Key :type Key%20Structure :default "None"))
  ;[1 1 1] debug set team
  (:Pressed
    (bind _asbasketball_player_state_bp (Utilities|Casting|CastToBasketballPlayerState_BP (Variables|GetPlayerState)))
    (Default|SetTeam _asbasketball_player_state_bp self (Utilities|Select :Index (Variables|/Game/BasketballTemplate/BasketballPlayerState_BP.BasketballPlayerState_BP_C|GetTeamId _asbasketball_player_state_bp) :Option%200 1 :Option%201 0))))

(event Input|KeyboardEvents|8
  (params (Key :type Key%20Structure :default "None"))
  (:Pressed
    (Default|CallDebug)))

(fn ConstructionScript)

(fn OnRepInputKeysBlocker
  (CallFunction|RecheckInputPossibility))

(fn OnRepOutOfBoundAfterBasket
  (if (Variables|Default|GetOutOfBoundAfterBasket)
    (Class|CharacterActionsInterfaceBP|SetMovementConstrain(Message) (Pawn|GetControlledPawn) true "X")
    (else
      (Class|CharacterActionsInterfaceBP|SetMovementConstrain(Message) (Pawn|GetControlledPawn) false "Custom"))))

(fn GetBall
  (return (Variables|/Game/BasketballTemplate/GameSettingsActor_BP.GameSettingsActor_BP_C|GetBall (Variables|Default|GetGameSettings))))

(fn GetEnemies
  (bind _gamesettings (Variables|Default|GetGameSettings))
  (bind _team1 (Variables|/Game/BasketballTemplate/GameSettingsActor_BP.GameSettingsActor_BP_C|GetTeam1 _gamesettings))
  (return (select (Utilities|Array|ContainsItem _team1 (Pawn|GetControlledPawn)) (Variables|/Game/BasketballTemplate/GameSettingsActor_BP.GameSettingsActor_BP_C|GetTeam2 _gamesettings) _team1)))

(fn GetHoops
  (return (Variables|/Game/BasketballTemplate/GameSettingsActor_BP.GameSettingsActor_BP_C|GetHoops (Variables|Default|GetGameSettings))))

(fn GetTeam
  (bind _gamesettings (Variables|Default|GetGameSettings))
  (bind _team1 (Variables|/Game/BasketballTemplate/GameSettingsActor_BP.GameSettingsActor_BP_C|GetTeam1 _gamesettings))
  (return (select (Utilities|Array|ContainsItem _team1 (Pawn|GetControlledPawn)) _team1 (Variables|/Game/BasketballTemplate/GameSettingsActor_BP.GameSettingsActor_BP_C|GetTeam2 _gamesettings))))

(fn Inited
  (return (Utilities|IsValid (Variables|Default|GetGameSettings))))